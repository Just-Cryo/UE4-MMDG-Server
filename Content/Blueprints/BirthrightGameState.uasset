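; BirthrightGameState is the replicated game state for a two-player, turn-based puzzle match, holding player data, start state and whose turn it is.
; A delayed update copies each PuzzlePlayerController's name and Elo into Player 1 or 2 data by array order.
; On the authority, StartGame and NextTurn set or flip the turn and tell PuzzleGameMode which player index begins the new turn.
; Several RepNotify handlers are empty or only print debug text.
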(event `ROS_UpdatePlayerInfo`
  (`KismetSystemLibrary.Delay` 1.0)
  (bind _outactors (`GameplayStatics.GetAllActorsOfClass` "/Game/PuzzleBP/Blueprints/PuzzlePlayerController.PuzzlePlayerController_C"))
  (for (_array_element _array_index) _outactors
    (if (== _array_index 0)
      (bind _name (`/Game/PuzzleBP/Blueprints/PuzzlePlayerController.Name` _array_element))
      (bind _elo (`/Game/PuzzleBP/Blueprints/PuzzlePlayerController.Elo` _array_element))
      (set `self.Player1Data` (make `/Game/Blueprints/PlayerInfo` _name _elo))
      (else
        (set `self.Player2Data` (make `/Game/Blueprints/PlayerInfo` _name _elo))))
    (`KismetSystemLibrary.PrintString` (`KismetStringLibrary.Concat_StrStr` "SET PLAYER DATA !!!!!!!!!!!!!!!!!!!!!!!!!!!!!!!!!!!!!!!!!!!!!!!!!!!!!!!!!!!!!!!!!!!!!!!!!!!!!!!!!!!!!!!!!!!!!!!!! \n" "NAme: " _name "Index: " (`KismetStringLibrary.Conv_IntToString` _array_index)))
    (set `self.Help` "AAAAAAAAAAAAAAAAAAAAAAAAAAAAAAAAAAAAAAAAAAAAAAAAAA"))
  (`KismetSystemLibrary.PrintString` (`KismetStringLibrary.Concat_StrStr` "COMPLETED ALL!!!!!!!!!!!!!!" (`KismetStringLibrary.Conv_IntToString` (`KismetArrayLibrary.Array_Length` _outactors)))))

(event `StartGame`
  (`/Engine/EditorBlueprintResources/ActorMacros.Switch Has Authority`
    (:`Authority`
      (set `self.GameStarted` true)
      (set `self.Player1Turn` true)
      (bind _aspuzzle_game_mode (cast `/Game/PuzzleBP/Blueprints/PuzzleGameMode` (`GameplayStatics.GetGameMode`)))
      (`/Game/PuzzleBP/Blueprints/PuzzleGameMode.ROS_NewTurn` _aspuzzle_game_mode 0))))

(event `NextTurn`
  (`/Engine/EditorBlueprintResources/ActorMacros.Switch Has Authority`
    (:`Authority`
      (bind _output_get (set `self.Player1Turn` (not (`self.Player1Turn`))))
      (bind _aspuzzle_game_mode (cast `/Game/PuzzleBP/Blueprints/PuzzleGameMode` (`GameplayStatics.GetGameMode`)))
      (`/Game/PuzzleBP/Blueprints/PuzzleGameMode.ROS_NewTurn` _aspuzzle_game_mode (`KismetMathLibrary.SelectInt` 0 1 _output_get)))))

(fn `GetPlayerData`
  (params (`Player 1` :type Boolean))
  (returns (`Player Data` :type "/Game/Blueprints/PlayerInfo Structure"))
  (return (select `bool` `Player 1` :`false` (`self.Player2Data`) :`true` (`self.Player1Data`))))

(fn `OnRep_GameStarted`)

(fn `OnRep_Help`
  (`KismetSystemLibrary.PrintString` "Updated Help"))

(fn `OnRep_Player1Turn`)

(fn `OnRep_PlayersData`
  (`KismetSystemLibrary.PrintString` (`KismetStringLibrary.Concat_StrStr` "PlayerData Modified!  \n" (`KismetStringLibrary.Conv_IntToString` (`KismetArrayLibrary.Array_Length` (`self.PlayersData`))))))

(fn `UserConstructionScript`
  (bind _playersdata (`self.PlayersData`))
  (`KismetArrayLibrary.Array_Set` _playersdata 0 (make `/Game/Blueprints/PlayerInfo` "Player 1") true)
  (`KismetArrayLibrary.Array_Set` _playersdata 1 (make `/Game/Blueprints/PlayerInfo` "Player 2") true))